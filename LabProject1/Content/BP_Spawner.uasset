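; BP_Spawner is a spawner actor that scatters random coins across the level when play begins.
; BeginPlay finds every TargetPoint tagged "SpawnPoint" and spawns a random CoinTypes entry at each one's transform.
; A SpawnPoint event spawns BP_Cube at a random position in a fixed range, but its looping timer is disconnected.
; Alternative BP_Coin spawns using the SpawnPositions array are also left unwired.
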(event `self.ReceiveBeginPlay`
  (bind _outactors (`GameplayStatics.GetAllActorsOfClassWithTag` "/Script/Engine.TargetPoint" "SpawnPoint"))
  (for _array_element _outactors
    (`|SpawnActorFromClass` (`|GetArrayItem` (`self.CoinTypes`) (`KismetMathLibrary.RandomIntegerInRange` 0 (- (`KismetArrayLibrary.Array_Length` (`self.CoinTypes`)) 1))) (`self.GetTransform` _array_element) "Undefined" "MultiplyWithRoot" null null)))

(event `SpawnPoint`
  (`|SpawnActorFromClass` "/Game/BP_Cube.BP_Cube_C" (`KismetMathLibrary.Conv_VectorToTransform` (`KismetMathLibrary.MakeVector` (`KismetMathLibrary.RandomFloatInRange` 500.0 2500.0) (`KismetMathLibrary.RandomFloatInRange` 1000.0 2000.0) (`KismetMathLibrary.RandomFloatInRange` 100.0 800.0))) "Undefined" "MultiplyWithRoot" null null))

(fn `UserConstructionScript`)