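; BP_EnemyAIController is an AI controller that drives a BP_EnemyAIPawn through patrol, chase and investigate behavior.
; After a short startup delay it caches the pawn and loops through its patrol points with AIMoveTo.
; When AIPerception senses an actor, the pawn speeds up and chases it.
; When the stimulus is lost, it slows, moves to the last sensed location, pauses, then resumes patrol.
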(event `self.ReceiveBeginPlay`
  (`KismetSystemLibrary.Delay` 0.5)
  (bind _asbp_enemy_aipawn (cast `/Game/CustomAI/BP_EnemyAIPawn` (`self.K2_GetPawn`)))
  (set `self.PawnRef` _asbp_enemy_aipawn)
  (`self.Patrol`))

(event `Patrol`
  (bind _pawnref (`self.PawnRef`))
  (`|AIMoveTo` _pawnref (`self.K2_GetActorLocation` (`|GetArrayItem` (`/Game/CustomAI/BP_EnemyAIPawn.PatrolPoints` _pawnref) (`/Game/CustomAI/BP_EnemyAIPawn.CurrentPatrolIndex` _pawnref))) null
    (:`OnSuccess`
      (`/Game/CustomAI/BP_EnemyAIPawn.GetNextPatrolPoint` (`self.PawnRef`))
      (`self.Patrol`))))

(event `self.AIPerception.OnTargetPerceptionUpdated`
  (params (Actor :type "Actor Object Reference") (Stimulus :type "AIStimulus Structure"))
  (bind (_age _expirationage _strength _stimuluslocation _receiverlocation _tag _bsuccessfullysensed) (break `AIStimulus` Stimulus))
  (if _bsuccessfullysensed
    (bind _output_get (set `self.TargetActor` Actor))
    (`self.StopMovement`)
    (set `CharacterMovementComponent.MaxWalkSpeed` 400.0 (`Character.CharacterMovement` (`self.PawnRef`)))
    (`|AIMoveTo` (`self.PawnRef`) (0.0 0.0 0.0) _output_get)
    (else
      (set `CharacterMovementComponent.MaxWalkSpeed` 200.0 (`Character.CharacterMovement` (`self.PawnRef`)))
      (set `self.TargetActor` null)
      (`|AIMoveTo` (`self.PawnRef`) _stimuluslocation null
        (:`OnSuccess`
          (`KismetSystemLibrary.Delay` 3.0)
          (`self.Patrol`))))))

(fn `UserConstructionScript`)