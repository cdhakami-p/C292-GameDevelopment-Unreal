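; BP_Light is a light actor that switches off when its matching target is hit.
; On BeginPlay it scans all BP_Target actors and binds to the OnTargetHit dispatcher of those whose IdTarget equals its IdLight.
; When that event fires, LightOff sets the point light's intensity to zero, with no path to turn it back on.
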(event `self.ReceiveBeginPlay`
  (bind _outactors (`GameplayStatics.GetAllActorsOfClass` "/Game/BP_Target.BP_Target_C"))
  (for _array_element _outactors
    (bind _asbp_target (cast `/Game/BP_Target` _array_element))
    (if (== (`self.id_light`) (`/Game/BP_Target.id_target` _asbp_target))
      (add `/Game/BP_Target.OnTargetHit` _asbp_target (delegate `LightOff`)))))

(event `LightOff`
  (`LightComponent.SetIntensity` (`self.PointLight`) 0.0))

(fn `UserConstructionScript`)