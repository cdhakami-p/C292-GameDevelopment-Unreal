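; BP_Pit is an actor that reveals its Plane component when a linked target is hit.
; On BeginPlay it searches all BP_Target actors for those whose IdTarget matches its own IdPit and binds PitOpen to their OnTargetHit event.
; PitOpen only makes the Plane visible, without propagating to child components.
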(event `self.ReceiveBeginPlay`
  (bind _outactors (`GameplayStatics.GetAllActorsOfClass` "/Game/BP_Target.BP_Target_C"))
  (for _array_element _outactors
    (bind _asbp_target (cast `/Game/BP_Target` _array_element))
    (if (== (`/Game/BP_Target.id_target` _asbp_target) (`self.id_pit`))
      (add `/Game/BP_Target.OnTargetHit` _asbp_target (delegate `Pit Open`)))))

(event `Pit Open`
  (`SceneComponent.SetVisibility` (`self.Plane`) true false))

(fn `UserConstructionScript`)